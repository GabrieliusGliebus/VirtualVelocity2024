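; Race start/finish line that counts laps for the player and opponent and ends the race when either exceeds the lap limit from MainGameInstance.
; Tick uses a Delay as a one-second clock for lap and total time.
; NewLap overlaps count player laps on entry and opponent laps on exit, resetting lap time only when it misses the best.
; Finishing writes best and total times to the game instance, then opens MainMenu.
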(event OnComponentBeginOverlap(NewLap)
  (params (OverlappedComponent :type Primitive%20Component%20Object%20Reference) (OtherActor :type Actor%20Object%20Reference) (OtherComp :type Primitive%20Component%20Object%20Reference) (OtherBodyIndex :type Integer) (bFromSweep :type Boolean) (SweepResult :type Hit%20Result%20Structure%20%28by%20ref%29))
  (if (Actor|ActorHasTag OtherActor "Player")
    (Variables|Laps|SetLapCount (+ (Variables|Laps|GetLapCount) 1))
    (if (< (Variables|Default|GetLapSeconds) (Variables|Default|GetBestLapSeconds))
      (Variables|Default|SetBestLapSeconds (Variables|Default|GetLapSeconds))
      (else
        (Variables|Default|SetLapSeconds 0)))
    (if (> (Variables|Laps|GetLapCount) (Variables|Laps|GetMaxLaps))
      (CallFunction|FinishGame))))

(event OnComponentEndOverlap(NewLap)
  (params (OverlappedComponent :type Primitive%20Component%20Object%20Reference) (OtherActor :type Actor%20Object%20Reference) (OtherComp :type Primitive%20Component%20Object%20Reference) (OtherBodyIndex :type Integer))
  (if (Actor|ActorHasTag OtherActor "Opponent")
    (bind _output_get (Variables|Laps|SetOpponent%20lap%20count (+ (Variables|Laps|GetOpponent%20lap%20count) 1)))
    (Development|PrintString (Utilities|String|BuildString(Integer) "Opponent " "" _output_get))
    (if (> (Variables|Laps|GetOpponent%20lap%20count) (Variables|Laps|GetMaxLaps))
      (CallFunction|FinishGame))))

(event Custom|FinishGame
  (CallFunction|BestS2M)
  (bind _asmain_game_instance (Utilities|Casting|CastToMainGameInstance (Game|GetGameInstance)))
  (Variables|/Game/MapsAndLevels/MainGameInstance.MainGameInstance_C|SetSelectedPawn _asmain_game_instance 0)
  (Variables|/Game/MapsAndLevels/MainGameInstance.MainGameInstance_C|SetBestSeconds _asmain_game_instance (Variables|Default|GetBestLapSeconds))
  (Variables|/Game/MapsAndLevels/MainGameInstance.MainGameInstance_C|SetBestMinutes _asmain_game_instance (Variables|Default|GetBestLapMinutes))
  (Variables|/Game/MapsAndLevels/MainGameInstance.MainGameInstance_C|SetTotalMinutes _asmain_game_instance (Variables|TotalTime|GetTotalTimeMinutes))
  (Variables|/Game/MapsAndLevels/MainGameInstance.MainGameInstance_C|SetTotalSeconds _asmain_game_instance (Variables|TotalTime|GetTotalTimeSeconds))
  (Utilities|FlowControl|Delay 1.0)
  (Variables|/Game/MapsAndLevels/MainGameInstance.MainGameInstance_C|SetHasTheGameFinished? _asmain_game_instance true)
  (Game|OpenLevel(byObjectReference) "/Game/MapsAndLevels/MainMenu.MainMenu"))

(event Custom|BestS2M
  (while (>= (Variables|Default|GetBestLapSeconds) 60)
    (Variables|Default|SetBestLapSeconds (- (Variables|Default|GetBestLapSeconds) 60))
    (Variables|Default|SetBestLapMinutes (+ (Variables|Default|GetBestLapMinutes) 1))))

(event EventBeginPlay
  (bind _asmain_game_instance (Utilities|Casting|CastToMainGameInstance (Game|GetGameInstance)))
  (Variables|Laps|SetMaxLaps (Variables|/Game/MapsAndLevels/MainGameInstance.MainGameInstance_C|GetNumberOfLaps _asmain_game_instance)))

(event EventTick
  (params (DeltaSeconds :type Float%20%28single-precision%29))
  (switch int (Variables|Laps|GetLapCount)
    (:Default
      (Utilities|FlowControl|Delay 1.0)
      (Variables|Default|SetLapSeconds (+ (Variables|Default|GetLapSeconds) 1))
      (Variables|TotalTime|SetTotalTimeSeconds (+ (Variables|TotalTime|GetTotalTimeSeconds) 1))
      (if (== (Variables|TotalTime|GetTotalTimeSeconds) 60)
        (Variables|TotalTime|SetTotalTimeSeconds 0)
        (Variables|TotalTime|SetTotalTimeMinutes (+ (Variables|TotalTime|GetTotalTimeMinutes) 1))))))

(fn ConstructionScript)