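; Starting-lights Blueprint that plays a timed visual and audio countdown, likely for a race start.
; On BeginPlay, a linear chain of delays reveals red, yellow and green lights one at a time, each with a short low beep.
; It then hides all three, shows a separate green light with a long high tone, and later hides that light.
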(event EventBeginPlay
  (Utilities|FlowControl|Delay 3.0)
  (Audio|PlaySound2D "/Game/MusicAndSounds/LowShort.LowShort" 1.0 1.0 0.0 0 0)
  (Rendering|SetVisibility (Variables|RedLight|GetRedLight1) true true)
  (Utilities|FlowControl|Delay 1.0)
  (Rendering|SetVisibility (Variables|YellowLights|GetYellowLight1) true true)
  (Audio|PlaySound2D "/Game/MusicAndSounds/LowShort.LowShort" 1.0 1.0 0.0 0 0)
  (Utilities|FlowControl|Delay 1.0)
  (Rendering|SetVisibility (Variables|GreenLightsMid|GetGreenLight1) true true)
  (Audio|PlaySound2D "/Game/MusicAndSounds/LowShort.LowShort" 1.0 1.0 0.0 0 0)
  (Utilities|FlowControl|Delay 1.0)
  (Rendering|SetVisibility (Variables|GreenLightsMid|GetGreenLight1) false true)
  (Rendering|SetVisibility (Variables|GreenLightsLow|GetLowGreen1) true true)
  (Audio|PlaySound2D "/Game/MusicAndSounds/HighLong.HighLong" 1.0 1.0 0.0 0 0)
  (Utilities|FlowControl|Delay 15.0)
  (Rendering|SetVisibility (Variables|GreenLightsLow|GetLowGreen1) false true))

(fn ConstructionScript)