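; BP_MainMenu is a menu actor that shows a widget and hands the view over to other linked menu actors.
; On BeginPlay it binds to the TransitionToLinkedMenu dispatcher of its WS_BaseClass widget, whose index selects an entry in LinkedMenus.
; A transition hides and disables collision on this actor, eases the player view to the revealed target menu, and enables that menu's collision after a delay matching the blend.
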(event Custom|TransitionTo
  (params (NewMenu :type BP%20Main%20Menu%20Object%20Reference))
  (Collision|SetActorEnableCollision false)
  (Rendering|SetActorHiddenInGame true)
  (Game|Player|SetViewTargetwithBlend (Game|GetPlayerController 0) NewMenu 2.0 "VTBlend_EaseInOut" 2.0 false)
  (Rendering|SetActorHiddenInGame NewMenu false)
  (Utilities|FlowControl|Delay 2.0)
  (Collision|SetActorEnableCollision NewMenu true))

(event Custom|TransitionToLinkedMenu_Event
  (params (MenuIndex :type Integer))
  (if (Utilities|Array|IsValidIndex (Variables|Default|GetLinkedMenus) MenuIndex)
    (CallFunction|Transitionto (Utilities|Array|Get(acopy) (Variables|Default|GetLinkedMenus) MenuIndex))))

(event EventBeginPlay
  (bind _asws_base_class (Utilities|Casting|CastToWS_BaseClass (UserInterface|GetUserWidgetObject (Variables|Default|GetWidget))))
  (EventDispatchers|AssignTransitiontoLinkedMenu _asws_base_class (delegate Custom|TransitionToLinkedMenu_Event)))

(fn ConstructionScript)