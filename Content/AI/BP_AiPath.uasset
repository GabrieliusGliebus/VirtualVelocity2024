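; BP_AiPath is a spline path actor that supplies road-side target locations for AI to follow.
; GetClosestLocationToPath finds the spline point nearest the AI, advances it by an additional distance, then shifts it along the spline's right vector to the chosen side of the road.
; The lateral offset is a fixed amount either way, and the actor runs no event or construction logic of its own.
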(event EventBeginPlay)

(event Collision|EventActorBeginOverlap
  (params (OtherActor :type Actor%20Object%20Reference)))

(event EventTick
  (params (DeltaSeconds :type Float%20%28single-precision%29)))

(fn ConstructionScript)

(fn GetClosestLocationtoPath
  (params (AILocation :type Vector :default "0, 0, 0") (Additional%20Distance :type Float%20%28double-precision%29) (SideOfRoad :type Integer))
  (bind _splinepath (Variables|Default|GetSplinePath))
  (bind _returnvalue (Class|SplineComponent|FindInputKeyClosesttoWorldLocation _splinepath AILocation))
  (bind _returnvalue_2 (Class|SplineComponent|GetDistanceAlongSplineatSplineInputKey _splinepath _returnvalue))
  (bind _returnvalue_3 (+ _returnvalue_2 Additional%20Distance))
  (return (+ (Spline|GetLocationatDistanceAlongSpline (Variables|Default|GetSplinePath) _returnvalue_3 "World") (* (Class|SplineComponent|GetRightVectoratDistanceAlongSpline (Variables|Default|GetSplinePath) _returnvalue_3 "World") (Math|Float|SelectFloat 4e+02 -4e+02 (Math|Conversions|ToBoolean(Integer) SideOfRoad))))))