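; BP_OpponentSpawner spawns a single AI car opponent when play begins, at one of four possible locations.
; BeginPlay picks a random index and passes the matching spawn-location component to SpawnTheOpponent.
; That function spawns PWN_AiCar at the component's world position with a fixed half-turn rotation, adjusting for collisions but always spawning.
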(event EventBeginPlay
  (switch int (Math|Random|RandomIntegerinRange 0 3)
    (:0
      (CallFunction|SpawntheOpponent (Variables|Default|GetOpponentSpawnLocation0)))
    (:1
      (CallFunction|SpawntheOpponent (Variables|Default|GetOpponentSpawnLocation1)))
    (:2
      (CallFunction|SpawntheOpponent (Variables|Default|GetOpponentSpawnLocation2)))
    (:3
      (CallFunction|SpawntheOpponent (Variables|Default|GetOpponentSpawnLocation3)))))

(event Collision|EventActorBeginOverlap
  (params (OtherActor :type Actor%20Object%20Reference)))

(event EventTick
  (params (DeltaSeconds :type Float%20%28single-precision%29)))

(fn ConstructionScript)

(fn SpawntheOpponent
  (params (SpawnLocation :type Scene%20Component%20Object%20Reference))
  (Game|SpawnActorfromClass "/Game/AI/PWN_AiCar.PWN_AiCar_C" (Math|Transform|MakeTransform (Transformation|GetWorldLocation SpawnLocation) "0.000000,180.000000,0.000000") "AdjustIfPossibleButAlwaysSpawn" "MultiplyWithRoot" 0 0))