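; SUV vehicle child Blueprint that adds an in-car minimap display and applies the saved paint color.
; On BeginPlay it runs the parent logic, creates a WB_Minimap widget for the MinimapScreen component, then reads SUVSavedColor from MainGameInstance.
; A selection macro maps that index to black, white, green or blue helpers, each swapping the mesh's first material slot.
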(event EventBeginPlay
  (|CallParentFunction)
  (bind _returnvalue (UserInterface|CreateWidget "/Game/Cameras/Minimap/WB_Minimap.WB_Minimap_C"))
  (bind _output_get (Variables|Default|SetActiveMinimap _returnvalue))
  (UserInterface|SetWidget (Variables|Default|GetMinimapScreen) _output_get)
  (bind _asmain_game_instance (Utilities|Casting|CastToMainGameInstance (Game|GetGameInstance)))
  (|setcolorsuv_2 self (Variables|/Game/MapsAndLevels/MainGameInstance.MainGameInstance_C|GetSUVSavedColor _asmain_game_instance)))

(event Collision|EventActorBeginOverlap
  (params (OtherActor :type Actor%20Object%20Reference)))

(event EventTick
  (params (DeltaSeconds :type Float%20%28single-precision%29)))

(fn ConstructionScript
  (|CallParentFunction))